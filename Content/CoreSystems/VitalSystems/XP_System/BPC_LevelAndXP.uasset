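; Actor component that tracks XP and level, handles level-ups and keeps an XP widget in sync.
; IncreaseXP adds XP and, at the cap, levels up, resets current XP and recursively applies the leftover.
; Each level raises max XP by 25 percent, truncated.
; Changes fire dispatchers bound on BeginPlay that message the widget, which SetStartingXPValues stores and seeds with starting values.
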(event `self.ReceiveBeginPlay`
  (add `self.OnXPChanged` (delegate `OnXPChanged_Event`))
  (add `self.OnlevelChanged` (delegate `OnlevelChanged_Event`))
  (add `self.OnMaxXpChanged` (delegate `OnMaxXpChanged_Event`))
  (add `self.OnCurrentXpChanged` (delegate `OnCurrentXpChanged_Event`)))

(event `OnMaxXpChanged_Event` :!signature `self.OnMaxXpChanged`
  (params (NewMaxXp :type "Float (double-precision)"))
  (message `/Game/CoreSystems/VitalSystems/XP_System/BPI_XP_widget.SetMaxXp` (`self.XP_widget`) NewMaxXp))

(event `OnCurrentXpChanged_Event` :!signature `self.OnCurrentXpChanged`
  (params (CurrentXP :type "Float (double-precision)"))
  (message `/Game/CoreSystems/VitalSystems/XP_System/BPI_XP_widget.SetCurrentXP` (`self.XP_widget`) CurrentXP))

(event `OnXPChanged_Event` :!signature `self.OnXPChanged`
  (params (NewXPPercentage :type "Float (double-precision)"))
  (message `/Game/CoreSystems/VitalSystems/XP_System/BPI_XP_widget.SetXpPercentage` (`self.XP_widget`) NewXPPercentage))

(event `OnlevelChanged_Event` :!signature `self.OnlevelChanged`
  (params (NewLevel :type Integer))
  (message `/Game/CoreSystems/VitalSystems/XP_System/BPI_XP_widget.SetLevelNumber` (`self.XP_widget`) NewLevel))

(fn `CalculateXPPercentage`
  ;[1 1 1] Calculates the xp percentage for the ui
  (`self.OnXPChanged` (`KismetMathLibrary.SafeDivide` (`self.CurrentXP`) (`self.MaxXP`))))

(fn `IncreaseLevel`
  (bind _result (`/Engine/EditorBlueprintResources/StandardMacros.IncrementInt` (`self.Level`))
    (:`  `
      (`self.OnlevelChanged` _result)
      (`self.IncreaseMaxXp`))))

(fn `IncreaseMaxXp`
  (bind _output_get (set `self.MaxXP` (`KismetMathLibrary.Conv_IntToDouble` (`KismetMathLibrary.FTrunc` (* (`self.MaxXP`) 1.25)))))
  (`self.OnMaxXpChanged` _output_get)
  (`self.CalculateXPPercentage`))

(fn `IncreaseXP`
  (params (AmountToIncreaseBy :type "Float (double-precision)"))
  (locals (LLeftOverXp :type "Float (double-precision)"))
  ;[1 1 1] Add incoming XP to current XP
  (set `self.CurrentXP` (+ (`local.AmountToIncreaseBy`) (`self.CurrentXP`)))
  ;[1 1 1] Call to update ui on new xp value
  (`self.OnCurrentXpChanged` (`self.CurrentXP`))
  ;[1 1 1] Calculate new percentage
  (`self.CalculateXPPercentage`)
  ;[1 1 1] Check if current xp is more than max xp
  (if (>= (`self.CurrentXP`) (`self.MaxXP`))
    ;[1 1 1] calculate left over xp
    (set `local.LLeftOverXp` (- (`self.CurrentXP`) (`self.MaxXP`)))
    ;[1 1 1] Increase xp updates ui and max xp
    (`self.IncreaseLevel`)
    ;[1 1 1] set current xp back to zero and run through the add xp function again until dont have more xp thean levels
    (set `self.CurrentXP` 0.0)
    (`self.IncreaseXP` (`local.LLeftOverXp`))))

(fn `SetStartingXPValues`
  (params (XP_widget :type "UserWidget Object Reference"))
  (set `self.XP_widget` XP_widget)
  ;[1 1 1] Sets starting xp values if not full
  (`self.OnlevelChanged` (`self.Level`))
  (`self.OnMaxXpChanged` (`self.MaxXP`))
  (`self.OnCurrentXpChanged` (`self.CurrentXP`))
  (`self.CalculateXPPercentage`))