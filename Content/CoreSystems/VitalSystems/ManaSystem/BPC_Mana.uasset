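; Actor component that manages a character's mana pool: spending, regenerating, raising the maximum and driving a mana bar.
; UseMana rejects insufficient mana; otherwise it deducts the cost, stops regen and restarts it after a retriggerable delay.
; A looping timer adds the regen rate until full, then clears itself.
; Changes broadcast the mana percentage through OnManaChanged, which updates the progress bar supplied by SetStartingManaValues.
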(event `self.ReceiveBeginPlay`
  (add `self.OnManaChanged` (delegate `SetManaBarPercent`)))

(event `SetManaBarPercent` :!signature `self.OnManaChanged`
  (params (NewPercentage :type "Float (double-precision)"))
  (bind _manaprogressbar (`self.ManaProgressBar`))
  (`/Engine/EditorBlueprintResources/StandardMacros.IsValid` _manaprogressbar
    (:`Is Valid`
      (message `/Game/CoreSystems/VitalSystems/MasterProgressBarWidget/BPI_vitalSystemsInterface.SetprogressBar` _manaprogressbar NewPercentage))
    (:`Is Not Valid`
      (`KismetSystemLibrary.PrintString` "Mana Progress Bar Not Valid"))))

(event `RegenMana`
  ;[1 1 1] controls how long before mana starts regening
  (`KismetSystemLibrary.RetriggerableDelay` 2.0)
  ;[1 1 1] reduces every 0.1 second
  (bind _returnvalue (`KismetSystemLibrary.K2_SetTimerDelegate` (delegate `RegenLoop`) 0.1 true))
  (set `self.TimerHandle` _returnvalue))

(event `RegenLoop`
  ;[1 1 1] Increase by the regen rate for mana
  (bind _manafull (`self.IncreaseMana` (`self.ManaRegenRate`)))
  (if _manafull
    (`KismetSystemLibrary.K2_ClearAndInvalidateTimerHandle` (`self.TimerHandle`))))

(fn `CalculateManaPercentage`
  ;[1 1 1] Calculate ths mana percentage
  (`self.OnManaChanged` (`KismetMathLibrary.SafeDivide` (`self.CurrentMana`) (`self.MaxMana`))))

(fn `IncreaseMana`
  (params (RegenRate :type "Float (double-precision)"))
  (returns (ManaFull :type Boolean))
  ;[1 1 1] Calculates percentage and stops going above max if at max returns full
  (bind _output_get (set `self.CurrentMana` (`KismetMathLibrary.FClamp` (+ (`self.CurrentMana`) RegenRate) 0.0 (`self.MaxMana`))))
  (`self.CalculateManaPercentage`)
  (if (>= _output_get (`self.MaxMana`))
    (return true)
    (else
      (return false))))

(fn `IncreaseMaxMana`
  (params (IncreasemaxManaBy :type "Float (double-precision)"))
  ;[1 1 1] Increase Max mana and re calcualte percentages
  (set `self.MaxMana` (+ (`self.MaxMana`) IncreasemaxManaBy))
  (`self.CalculateManaPercentage`))

(fn `SetStartingManaValues`
  (params (ManaProgressBar :type "UserWidget Object Reference"))
  ;[1 1 1] Sets values for events like save game
  (set `self.ManaProgressBar` ManaProgressBar)
  (`self.IncreaseMaxMana` 0.0)
  (`self.RegenMana`))

(fn `UseMana`
  (params (ManaToUse :type "Float (double-precision)"))
  (returns (Success :type Boolean))
  ;[1 1 1] checks if have enough mana to perform action if not exits out
  (if (>= (`self.CurrentMana`) ManaToUse)
    ;[1 1 1] If enough mana reduces the mana by requested amount clears timer make sure not regening and using at same time
    (`KismetSystemLibrary.K2_ClearAndInvalidateTimerHandle` (`self.TimerHandle`))
    (set `self.CurrentMana` (- (`self.CurrentMana`) (`local.ManaToUse`)))
    ;[1 1 1] calculates percentage and starts regen mana
    (`self.CalculateManaPercentage`)
    (`self.RegenMana`)
    (return true)
    (else
      (return false))))