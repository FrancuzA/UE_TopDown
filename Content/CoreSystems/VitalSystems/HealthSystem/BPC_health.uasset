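; Health component that tracks damage, regeneration, damage over time and death for its owning actor.
; Owner damage lowers clamped health, and a retriggerable delay restarts looping-timer regeneration; regen and damage-over-time timers cancel each other.
; OnHealthChanged updates a progress bar, either passed in or created as a screen-space widget above enemies and objects.
; OnDead ragdolls any skeletal mesh, removes that widget and clears bindings and references.
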(event `self.ReceiveBeginPlay`
  (`self.InitComponents`)
  ;[1 1 1] Bind to on damage event and decrease health
  (add `Actor.OnTakeAnyDamage` (`self.GetOwner`) (delegate `RecievedAnyDamage`))
  ;[1 1 1] Bind to custom on death Dispatcher
  (add `self.OnDead` (delegate `OnDead_Event`))
  ;[1 1 1] Bind to on health change to update the widget
  (add `self.OnHealthChanged` (delegate `SetNewProgress`)))

(event `OnDead_Event` :!signature `self.OnDead`
  (params (Killer :type "Actor Object Reference"))
  ;[1 1 1] Bind to custom on death Dispatcher
  (`self.OwnersSkeletelMesh`
    (:`then`
      (`self.Ragdoll`))
    (:`else`
      _))
  (bind _enemyandobjectwidgetcomp (`self.EnemyAndObjectWidgetComp`)
    (:`then`
      (`self.K2_DestroyComponent` _enemyandobjectwidgetcomp (`self.GetOwner`)))
    (:`else`
      _))
  (`self.ClearReferences`))

(event `SetNewProgress` :!signature `self.OnHealthChanged`
  (params (NewPercentage :type "Float (double-precision)"))
  (bind _healthprogresssbar (`self.HealthprogresssBar`))
  ;[1 1 1] Bind to on health change to update the widget
  (`/Engine/EditorBlueprintResources/StandardMacros.IsValid` _healthprogresssbar
    (:`Is Valid`
      (message `/Game/CoreSystems/VitalSystems/MasterProgressBarWidget/BPI_vitalSystemsInterface.SetprogressBar` _healthprogresssbar NewPercentage))
    (:`Is Not Valid`
      (`KismetSystemLibrary.PrintString` "ProgressBarHasNotBeenInitiatedFromPlayer"))))

(event `RecievedAnyDamage`
  (params (DamagedActor :type "Actor Object Reference") (Damage :type "Float (single-precision)") (DamageType :type "DamageType Object Reference") (InstigatedBy :type "Controller Object Reference") (DamageCauser :type "Actor Object Reference"))
  ;[1 1 1] Bind to on damage event and decrease health
  (`/Engine/EditorBlueprintResources/StandardMacros.IsValid` DamageCauser
    (:`Is Valid`
      (`self.DecreaseHealth` Damage DamageCauser))
    (:`Is Not Valid`
      (`KismetSystemLibrary.PrintString` "Damage Causer not valid"))))

(event `RegenHealth`
  (params (RegenRate :type "Float (double-precision)"))
  ;[1 1 1] controls how long before Health starts regening
  (`KismetSystemLibrary.RetriggerableDelay` 2.0)
  (if (not (<= (`self.CurrentHealth`) 0.0))
    ;[1 1 1] reduces every 0.1 second
    (bind _returnvalue (`KismetSystemLibrary.K2_SetTimerDelegate` (delegate `RegenLoop`) 0.1 true))
    (set `self.RegenTimer` _returnvalue)))

(event `RegenLoop`
  ;[1 1 1] Increase by the regen rate for Health
  (bind _healthfull (`self.IncreaseHealth` (stale `RegenHealth` RegenRate)))
  (if _healthfull
    (`self.StopRegenTimer`)))

(event `DamageOverTime`
  (params (AmountToDecreaseBy :type "Float (double-precision)"))
  (`self.StopRegenTimer`)
  ;[1 1 1] reduces every 0.1 second
  (bind _returnvalue (`KismetSystemLibrary.K2_SetTimerDelegate` (delegate `DOTLoop`) 0.1 true))
  (set `self.DOTTimer` _returnvalue))

(event `DOTLoop`
  ;[1 1 1] Increase by the regen rate for Health
  (bind _dead (`self.DecreaseHealth` (stale `DamageOverTime` AmountToDecreaseBy)))
  (if _dead
    (`self.StopDOTTimer`)))

(fn `CalculateHealthPercentage`
  ;[1 1 1] Calculate ths mana percentage
  (`self.OnHealthChanged` (`KismetMathLibrary.SafeDivide` (`self.CurrentHealth`) (`self.MaxHealth`))))

(fn `ClearReferences`
  (clear `Actor.OnTakeAnyDamage` (`self.GetOwner`))
  (clear `self.OnHealthChanged`)
  (clear `self.OnDead`)
  (set `self.HealthprogresssBar` null)
  (set `self.OwnersSkeletelMesh` null)
  (set `self.CapsuleComponent` null)
  (set `self.EnemyAndObjectWidgetComp` null))

(fn `DecreaseHealth`
  (params (AmountToDecreaseBy :type "Float (double-precision)") (DamageCausedBy :type "Actor Object Reference"))
  (returns (Dead :type Boolean))
  ;[1 1 1] cancels the regen timer so not regening and decreasing ats ame time
  (`self.StopRegenTimer`)
  ;[1 1 1] Gets health and reduces the amount and calculates the percentage for the UI
  (bind _output_get (set `self.CurrentHealth` (`KismetMathLibrary.FClamp` (- (`self.CurrentHealth`) (`local.AmountToDecreaseBy`)) 0.0 (`self.MaxHealth`))))
  (`self.CalculateHealthPercentage`)
  (if (<= _output_get 0.0)
    ;[1 1 1] Calls the dead event to be handled seperatley could also be handled here as well but this component can be used for physical objects and characters implementing ragdoll in here wouldnt work for both for eaxample
    (`self.StopRegenTimer`)
    (`self.OnDead` (`local.DamageCausedBy`))
    (return true)
    (else
      ;[1 1 1] Calls the regen event which will hit the retrigable delay if on the loop
      (`self.RegenHealth` (`self.HealthRegenRate`))
      (return false))))

(fn `IncreaseHealth`
  (params (IncreasAmount :type "Float (double-precision)"))
  (returns (HealthFull :type Boolean))
  ;[1 1 1] Increases health stops going above max
  (`self.StopDOTTimer`)
  (bind _output_get (set `self.CurrentHealth` (`KismetMathLibrary.FClamp` (+ (`self.CurrentHealth`) IncreasAmount) 0.0 (`self.MaxHealth`))))
  (`self.CalculateHealthPercentage`)
  (if (>= _output_get (`self.MaxHealth`))
    (return true)
    (else
      (return false))))

(fn `IncreaseMaxHealth`
  (params (IncreasemaxManaBy :type "Float (double-precision)"))
  ;[1 1 1] Increase Max mana and re calcualte percentages
  (set `self.MaxHealth` (+ (`self.MaxHealth`) IncreasemaxManaBy))
  (`self.CalculateHealthPercentage`))

(fn `InitComponents`
  (bind _returnvalue (`Actor.GetComponentByClass` (`self.GetOwner`) "/Script/Engine.CapsuleComponent"))
  (bind _returnvalue_2 (`Actor.GetComponentByClass` (`self.GetOwner`) "/Script/Engine.SkeletalMeshComponent"))
  (`/Engine/EditorBlueprintResources/StandardMacros.IsValid` _returnvalue_2
    (:`Is Valid`
      (set `self.OwnersSkeletelMesh` _returnvalue_2))
    (:`Is Not Valid`
      _))
  (`/Engine/EditorBlueprintResources/StandardMacros.IsValid` _returnvalue
    (:`Is Valid`
      (set `self.CapsuleComponent` _returnvalue))
    (:`Is Not Valid`
      _))
  (return))

(fn `InitEnemyOrObjectHealth`
  (params (Class :type "UserWidget Class Reference"))
  (locals (CaosuleHalfHeight :type "Float (single-precision)" :default 0.0))
  (bind _returnvalue (`|CreateWidget` Class))
  (bind _output_get (set `self.HealthprogresssBar` _returnvalue))
  (bind _userwidget (message `/Game/CoreSystems/VitalSystems/MasterProgressBarWidget/BPI_vitalSystemsInterface.GetProgressBar` _output_get))
  (`self.SetHealthStartingValues` _userwidget)
  (`/Engine/EditorBlueprintResources/StandardMacros.IsValid` (`self.CapsuleComponent`)
    (:`Is Valid`
      (set `local.CaosuleHalfHeight` (`CapsuleComponent.CapsuleHalfHeight` (`self.CapsuleComponent`))))
    (:`Is Not Valid`
      _))
  (bind _returnvalue_2 (`|AddComponentByClass` (`self.GetOwner`) "/Script/UMG.WidgetComponent" false (`KismetMathLibrary.MakeTransform` (`KismetMathLibrary.MakeVector` 0.0 0.0 (+ (select `bool` (`KismetSystemLibrary.IsValid` (`self.CapsuleComponent`)) :`false` (* (.z (`.BoxExtent` (`Actor.GetActorBounds` (`self.GetOwner`) false false))) 2.0) :`true` (`local.CaosuleHalfHeight`) :!type "Float (double-precision)") (`self.HealthZOffset`))))))
  (set `self.EnemyAndObjectWidgetComp` _returnvalue_2)
  (`WidgetComponent.SetWidgetSpace` (`self.EnemyAndObjectWidgetComp`) "Screen")
  (`WidgetComponent.SetWidget` (`self.EnemyAndObjectWidgetComp`) (`self.HealthprogresssBar`))
  (`WidgetComponent.SetDrawSize` (`self.EnemyAndObjectWidgetComp`) (`self.WidgetSize`))
  (`self.CalculateHealthPercentage`))

(fn `Ragdoll`
  (`PrimitiveComponent.SetCollisionProfileName` (`self.OwnersSkeletelMesh`) "Ragdoll" true)
  (`PrimitiveComponent.SetSimulatePhysics` (`self.OwnersSkeletelMesh`) true)
  (`PrimitiveComponent.SetCollisionEnabled` (`self.CapsuleComponent`) "NoCollision"))

(fn `SetHealthStartingValues`
  (params (HealthprogresssBar :type "UserWidget Object Reference"))
  ;[1 1 1] Sets the starting values for health
  (set `self.HealthprogresssBar` HealthprogresssBar)
  (`self.IncreaseMaxHealth` 0.0)
  (`self.RegenHealth` (`self.HealthRegenRate`)))

(fn `StopDOTTimer`
  ;[1 1 1] Stops the damage over time timer
  (`KismetSystemLibrary.K2_ClearAndInvalidateTimerHandle` (`self.DOTTimer`)))

(fn `StopRegenTimer`
  ;[1 1 1] Stops regen timer cleaner here for use in owners bps
  (`KismetSystemLibrary.K2_ClearAndInvalidateTimerHandle` (`self.RegenTimer`)))